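; Grabbable ship wheel Blueprint in the ship controller folder, moved through a physics handle.
; GrabObject attaches the supplied handle to the Wheel component at the grab location, and ReleaseObject releases it.
; Tick prints the forward vector of the Wheel's relative rotation as debug output; the wheel's rotation drives nothing else in this Blueprint.
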(event `self.ReceiveBeginPlay`)

(event `/Game/Blueprints/PhysicsActorInterface.GrabObject`
  (params (Handler :type "PhysicsHandleComponent Object Reference") (GrabLocation :type "Vector Structure"))
  (`PhysicsHandleComponent.GrabComponentAtLocation` Handler (`self.Wheel`) "None" GrabLocation))

(event `/Game/Blueprints/PhysicsActorInterface.ReleaseObject`
  (params (Handler :type "PhysicsHandleComponent Object Reference"))
  (`PhysicsHandleComponent.ReleaseComponent` Handler))

(event `self.ReceiveTick`
  (params (DeltaSeconds :type "Float (single-precision)"))
  (`KismetSystemLibrary.PrintString` (`KismetStringLibrary.Conv_VectorToString` (`KismetMathLibrary.GetForwardVector` (`SceneComponent.RelativeRotation` (`self.Wheel`)))) true true (struct :`G` 0.66 :`B` 1.0 :`A` 1.0) DeltaSeconds))

(fn `UserConstructionScript`)