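; Physics-driven ship actor with throttle, turning and simple health, destroyed when repeated Life events drain its health.
; A looping timer moves forward throttle by axis input or toward a clamped target, which can be set by ratio.
; Tick counters spin with opposing torque, blends velocity toward forward vector times throttle, applies yaw torque and prints debug throttle values.
; A vertical throttle updater mirrors the forward one but is never called here.
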(event `Set Ship Forward Target Throttle Using Ratio`
  (params (Ratio :type "Float (double-precision)"))
  ;[1 1 1] Take a Ratio between -1 and 1, and set the Forward Target Throttle based on that value
  (if (> Ratio 0.0)
    (set `self.ForwardTargetThrottle` (* (`self.MaxForwardThrottle`) Ratio))
    (else
      (set `self.ForwardTargetThrottle` (* (* -1 Ratio) (`self.MaxReverseThrottle`))))))

(event `self.ReceiveBeginPlay`
  ;[1 1 1] Update Foward
  (`KismetSystemLibrary.K2_SetTimer` null "UpdateForwardThrottle" (`self.UpdateThrottleTickRate`) true))

(event `InputAxis|ShipForward`
  (params (AxisValue :type "Float (single-precision)"))
  ;[1 0.4493 0.3695] Debug Forward Manual Keyboard Input
  (set `self.ForwardThrottleInput` AxisValue))

(event `self.ReceiveTick`
  (params (DeltaSeconds :type "Float (single-precision)"))
  ;[1 1 1] Debug print
  (`KismetSystemLibrary.PrintString` (`KismetStringLibrary.Concat_StrStr` "Vertical Throttle: " (`KismetStringLibrary.Conv_DoubleToString` (`self.VerticalTargetThrottle`)) "     " "Forward Throttle: " (`KismetStringLibrary.Conv_DoubleToString` (`self.ForwardThrottleAmount`))) true true (struct :`R` 1.0 :`G` 0.184235 :`B` 0.253958 :`A` 1.0) DeltaSeconds)
  ;[1 1 1] Update Physics
  (`PrimitiveComponent.AddTorqueInDegrees` (`self.ShipBase`) (/ (`KismetMathLibrary.NegateVector` (`PrimitiveComponent.GetPhysicsAngularVelocityInDegrees` (`self.ShipBase`) "None")) 0.5) "None" true)
  (`self.UpdateCalculatedSpeed`)
  ;[1 1 1] Update Turn w/ Debug Turn Manual Keyboard Input
  (set `self.TurnInput` (stale `InputAxis|ShipRight` AxisValue) :!label _label)
  (`self.UpdateTurning`))

(event `InputAxis|ShipRight`
  (params (AxisValue :type "Float (single-precision)"))
  ;[1 1 1] Update Turn w/ Debug Turn Manual Keyboard Input
  (goto _label))

(event `Death`
  ;[1 1 1] Health
  (`self.K2_DestroyActor`))

(event `Life`
  ;[1 1 1] Health
  (bind _output_get (set `self.ShipHealth` (- (`self.ShipHealth`) 25)))
  (`KismetSystemLibrary.PrintString` (`KismetStringLibrary.Conv_IntToString` _output_get))
  (if (<= (`self.ShipHealth`) 0)
    (`self.Death`)))

(fn `UpdateCalculatedSpeed`
  (bind _shipbase (`self.ShipBase`))
  (bind _returnvalue (`PrimitiveComponent.GetPhysicsLinearVelocity` _shipbase "None"))
  (`PrimitiveComponent.SetPhysicsLinearVelocity` (`self.ShipBase`) (`KismetMathLibrary.VLerp` _returnvalue (* (`SceneComponent.GetForwardVector` _shipbase) (* (`self.ForwardThrottleAmount`) (`self.UE4_ForceConstant`))) 0.01) false "None"))

(fn `UpdateForwardThrottle`
  (bind _forwardtargetthrottle (`self.ForwardTargetThrottle`))
  (bind _maxreversethrottle (`self.MaxReverseThrottle`))
  (bind _maxforwardthrottle (`self.MaxForwardThrottle`))
  (bind _forwardtargetthrottle_2 (`self.ForwardTargetThrottle`))
  (bind _forwardthrottleamount (`self.ForwardThrottleAmount`))
  (bind _returnvalue (+ (* (`self.ForwardThrottleInput`) (`self.ForwardAcceleration`)) (`self.ForwardThrottleAmount`)))
  ;[1 1 1] Clamp Initial Target Value
  (set `self.ForwardTargetThrottle` (`KismetMathLibrary.FClamp` (`self.ForwardTargetThrottle`) (`self.MaxReverseThrottle`) (`self.MaxForwardThrottle`)))
  ;[0.7975 0.4754 1] Forward Target Throttle Value is being Used
  (if (== (`self.UseForwardTargetThrottle`) true)
    ;[0.4588 0.6941 1] Set Forward Input depending on the direction Throttle Amount needs to catch-up to Target Throttle
    (if (== _forwardtargetthrottle _forwardthrottleamount)
      (set `self.ForwardThrottleInput` 0.0)
      ;[1 0.4583 0.4583] Simple Forward Throttle Update
      (set `self.ForwardThrottleAmount` (`KismetMathLibrary.FClamp` _returnvalue _maxreversethrottle _maxforwardthrottle) :!label _label)
      (elif (> _forwardtargetthrottle _forwardthrottleamount)
        (set `self.ForwardThrottleInput` 1.0)
        ;[0.4588 0.6941 1] Update Forward Throttle to its progress towards the Target, and also clamp it to the target
        (set `self.ForwardThrottleAmount` (`KismetMathLibrary.FClamp` _returnvalue _maxreversethrottle _forwardtargetthrottle_2))
        (else
          (set `self.ForwardThrottleInput` -1.0)
          (set `self.ForwardThrottleAmount` (`KismetMathLibrary.FClamp` _returnvalue _forwardtargetthrottle_2 _maxforwardthrottle)))))
    (else
      (goto _label))))

(fn `UpdateTurning`
  (bind _shipbase (`self.ShipBase`))
  (`PrimitiveComponent.AddTorqueInDegrees` _shipbase (`KismetMathLibrary.VLerp` (0.0 0.0 0.0) (* (`SceneComponent.GetUpVector` _shipbase) (* (`self.TurnInput`) (`self.TurnSpeed`))) (`self.TurnLerpAlpha`)) "None" true))

(fn `UpdateVerticalThrottle`
  (bind _verticaltargetthrottle (`self.VerticalTargetThrottle`))
  (bind _maxdownthrottle (`self.MaxDownThrottle`))
  (bind _verticalthrottleamount (`self.VerticalThrottleAmount`))
  (bind _maxupthrottle (`self.MaxUpThrottle`))
  (bind _verticaltargetthrottle_2 (`self.VerticalTargetThrottle`))
  (bind _returnvalue (+ (* (`self.VerticalTargetThrottle`) (`self.VerticalAcceleration`)) (`self.VerticalThrottleAmount`)))
  ;[1 1 1] Clamp Initial Target Value
  (set `self.VerticalTargetThrottle` (`KismetMathLibrary.FClamp` (`self.VerticalTargetThrottle`) (`self.MaxDownThrottle`) (`self.MaxUpThrottle`)))
  ;[0.7975 0.4754 1] Forward Target Throttle Value is being Used
  (if (== (`self.UseVerticalTargetThrottle`) true)
    ;[0.4588 0.6941 1] Set Forward Input depending on the direction Throttle Amount needs to catch-up to Target Throttle
    (if (== _verticaltargetthrottle _verticalthrottleamount)
      (set `self.VerticalThrottleInput` 0.0)
      ;[1 0.4583 0.4583] Simple Forward Throttle Update
      (set `self.VerticalTargetThrottle` (`KismetMathLibrary.FClamp` _returnvalue _maxdownthrottle _maxupthrottle) :!label _label)
      (elif (> _verticaltargetthrottle _verticalthrottleamount)
        (set `self.VerticalThrottleInput` 1.0)
        ;[0.4588 0.6941 1] Update Forward Throttle to its progress towards the Target, and also clamp it to the target
        (set `self.VerticalTargetThrottle` (`KismetMathLibrary.FClamp` _returnvalue _maxdownthrottle _verticaltargetthrottle_2))
        (else
          (set `self.VerticalThrottleInput` -1.0)
          (set `self.VerticalTargetThrottle` (`KismetMathLibrary.FClamp` _returnvalue _verticaltargetthrottle_2 _maxupthrottle)))))
    (else
      (goto _label))))

(fn `UserConstructionScript`)