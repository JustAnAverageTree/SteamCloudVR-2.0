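; Ship cannon actor that pitches up and down from axis input and fires projectiles.
; PitchCannon nudges the actor's pitch by scaled input, clamped to a fixed range while keeping roll and yaw.
; Firing is gated by CanFire: it spawns CannonProjectile_BP at the Barrel using the actor's rotation, then re-arms after a FireRate delay.
; ResetFire can also re-arm it but is not called here, and FireProjectile ignores its Direction input.
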(event `PitchCannon`
  (params (Axis :type "Float (double-precision)"))
  (bind (_returnvalue_roll _returnvalue_pitch _returnvalue_yaw) (`KismetMathLibrary.BreakRotator` (`self.K2_GetActorRotation`)))
  (`self.K2_SetActorRotation` (`KismetMathLibrary.MakeRotator` _returnvalue_roll (`KismetMathLibrary.FClamp` (+ (* Axis 0.1) _returnvalue_pitch) -20.0 30.0) _returnvalue_yaw)))

(event `self.ReceiveBeginPlay`)

(event `self.ReceiveTick`
  (params (DeltaSeconds :type "Float (single-precision)")))

(event `Firing`
  ;[1 1 1] Firing
  (if (`self.CanFire`)
    (set `self.CanFire` false)
    (`|ExecutionSequence`
      (:`then_0`
        (`self.Fire Projectile` (0.0 0.0 0.0)))
      (:`then_1`
        (`KismetSystemLibrary.Delay` (`self.FireRate`))
        (set `self.CanFire` true)))))

(fn `Fire Projectile`
  (params (Direction :type "Vector Structure"))
  ;[1 1 1] Spawn at location
  (`KismetSystemLibrary.PrintString` "here we go")
  (`|SpawnActorFromClass` "/Game/Blueprints/ShipController/CannonProjectile_BP.CannonProjectile_BP_C" (`KismetMathLibrary.MakeTransform` (`SceneComponent.K2_GetComponentLocation` (`self.Barrel`)) (`self.K2_GetActorRotation`)) "Undefined" "OverrideRootScale" null null))

(fn `ResetFire`
  (set `self.CanFire` true)
  (`KismetSystemLibrary.PrintString` "Hello"))

(fn `UserConstructionScript`)