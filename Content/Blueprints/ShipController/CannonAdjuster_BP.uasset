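; CannonAdjuster_BP is a grabbable lever control that adjusts the pitch of ship cannons.
; Grab and release events attach the Lever component to, or release it from, the calling handler.
; Each Tick, it reads the lever's world roll and calls PitchCannon on every cannon in its Cannons array, pitching one way or the other outside a dead zone around 90 degrees and passing zero inside it.
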(event `/Game/Blueprints/PhysicsActorInterface.GrabObject`
  (params (Handler :type "PhysicsHandleComponent Object Reference") (GrabLocation :type "Vector Structure"))
  (`PhysicsHandleComponent.GrabComponentAtLocation` Handler (`self.Lever`) "None" GrabLocation))

(event `/Game/Blueprints/PhysicsActorInterface.ReleaseObject`
  (params (Handler :type "PhysicsHandleComponent Object Reference"))
  (`PhysicsHandleComponent.ReleaseComponent` Handler))

(event `self.ReceiveTick`
  (params (DeltaSeconds :type "Float (single-precision)"))
  (bind _returnvalue_roll (`KismetMathLibrary.BreakRotator` (`SceneComponent.K2_GetComponentRotation` (`self.Lever`))))
  (for _array_element (`self.Cannons`)
    (if (<= _returnvalue_roll 85.0)
      (`/Game/Blueprints/ShipController/Cannon_BP.PitchCannon` _array_element 1.0)
      (elif (>= _returnvalue_roll 95.0)
        (`/Game/Blueprints/ShipController/Cannon_BP.PitchCannon` _array_element -1.0)
        (else
          (`/Game/Blueprints/ShipController/Cannon_BP.PitchCannon` _array_element 0.0))))))

(fn `UserConstructionScript`)