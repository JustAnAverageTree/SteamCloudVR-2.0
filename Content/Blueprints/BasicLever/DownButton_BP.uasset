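; DownButton_BP is a VR push button that a motion controller presses down along its local Z axis.
; While touched, Tick clamps the controller's height in actor space, offset by a third of the mesh height, between MaxDepth and zero; otherwise it lerps back up.
; Reaching or leaving MaxDepth calls empty hook functions for pressed, held and released, tracked with an IsPressedDown flag.
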(event `/Game/Blueprints/TouchActorInterface.TouchBegan`
  (params (ControllerScene :type "SceneComponent Object Reference") (Controller :type "MotionControllerComponent Object Reference"))
  (set `self.Motion Controller` Controller)
  (set `self.ControllerScene` ControllerScene))

(event `/Game/Blueprints/TouchActorInterface.TouchEnded`
  (set `self.Motion Controller` null)
  (set `self.ControllerScene` null))

(event `self.ReceiveBeginPlay`
  (set `self.MaxDepth` (* -1 (`self.MaxDepth`))))

(event `self.ReceiveTick`
  (params (DeltaSeconds :type "Float (single-precision)"))
  (bind _button (`self.Button`))
  (bind _ispresseddown (`self.isPressedDown`))
  (`|ExecutionSequence`
    (:`then_0`
      (`SceneComponent.K2_SetRelativeLocation` _button (`KismetMathLibrary.MakeVector` 0.0 0.0 (`self.CurrentButtonDepth`)) false false)
      (`/Engine/EditorBlueprintResources/StandardMacros.IsValid` (`self.Motion Controller`)
        (:`Is Valid`
          (set `self.CurrentButtonDepth` (`KismetMathLibrary.FClamp` (- (.z (`KismetMathLibrary.InverseTransformLocation` (`self.GetTransform`) (`SceneComponent.K2_GetComponentLocation` (`self.ControllerScene`)))) (/ (.z (`.Max` (break `Box` (`StaticMesh.GetBoundingBox` (`StaticMeshComponent.StaticMesh` _button))))) 3.0)) (`self.MaxDepth`) 0.0)))
        (:`Is Not Valid`
          (set `self.CurrentButtonDepth` (`KismetMathLibrary.Lerp` (`self.CurrentButtonDepth`) 0.0 (* (`self.LiftUpSpeed`) DeltaSeconds))))))
    (:`then_1`
      (if (== (`self.CurrentButtonDepth`) (`self.MaxDepth`))
        (if _ispresseddown
          (`self.Button Is Fully Down`)
          (else
            (`self.ButtonWasPressedFullyDown`)
            (set `self.isPressedDown` true)))
        (elif _ispresseddown
          (`self.Button Was Released from Being Full Down`)
          (set `self.isPressedDown` false))))))

(fn `Button Is Fully Down`)

(fn `Button Was Released from Being Full Down`)

(fn `ButtonWasPressedFullyDown`)

(fn `UserConstructionScript`)