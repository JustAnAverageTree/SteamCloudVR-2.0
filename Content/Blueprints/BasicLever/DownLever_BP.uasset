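; DownLever_BP is a VR lever that one or two motion controllers can grab and rotate about its hinge.
; Grabbing picks the nearest child collider of the lever, and Tick pins each hand to its collider.
; The primary controller's angle, offset by its collider's, sets the clamped lever roll.
; Empty grab, release and tick functions serve as hooks, alongside helpers for reading angle and stepped ratio.
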(event `/Game/Blueprints/PhysicsActorInterface.GrabObject`
  (params (Handler :type "PhysicsHandleComponent Object Reference") (GrabLocation :type "Vector Structure") (`Controller Scene` :type "SceneComponent Object Reference") (Controller :type "MotionControllerComponent Object Reference"))
  (bind _foundclosestcollider (`self.GetClosestCollider` `Controller Scene`))
  (if (== (`self.HandCount`) 0)
    (set `self.ClosestCollider` _foundclosestcollider)
    (`self.Grabbed`)
    (set `self.MotionController` Controller)
    (set `self.ControllerScene` `Controller Scene`)
    (else
      (set `self.ClosestCollider2` _foundclosestcollider)
      (set `self.MotionController2` Controller)
      (set `self.ControllerScene2` `Controller Scene`)))
  (`/Engine/EditorBlueprintResources/StandardMacros.IncrementInt` (`self.HandCount`)))

(event `/Game/Blueprints/PhysicsActorInterface.ReleaseObject`
  (params (Handler :type "PhysicsHandleComponent Object Reference") (`Controller Scene` :type "SceneComponent Object Reference"))
  (if (== (`self.HandCount`) 1)
    (`self.LetGoOf`)
    (set `self.MotionController` null)
    (set `self.ControllerScene` null)
    (set `self.ClosestCollider` null)
    (else
      (if (== `Controller Scene` (`self.ControllerScene`))
        (set `self.MotionController` (`self.MotionController2`))
        (set `self.ControllerScene` (`self.ControllerScene2`))
        (set `self.ClosestCollider` (`self.ClosestCollider2`)))
      (set `self.ClosestCollider2` null)
      (set `self.MotionController2` null)
      (set `self.ControllerScene2` null)))
  (`/Engine/EditorBlueprintResources/StandardMacros.DecrementInt` (`self.HandCount`)))

(event `self.ReceiveTick`
  (params (DeltaSeconds :type "Float (single-precision)"))
  (bind _motioncontroller2 (`self.MotionController2`))
  (`|ExecutionSequence`
    (:`then_0`
      (`self.TickUpdate`))
    (:`then_1`
      ;[1 1 1] Continue if Lever is Grabbed, and Update Hand Position to Grip
      (if (>= (`self.HandCount`) 1)
        (`|ExecutionSequence`
          (:`then_0`
            (`/Engine/EditorBlueprintResources/StandardMacros.IsValid` _motioncontroller2
              (:`Is Valid`
                (`self.UpdateHandPositionToCollider` _motioncontroller2 (`self.ClosestCollider2`)))))
          (:`then_1`
            (`self.UpdateHandPositionToCollider` (`self.MotionController`) (`self.ClosestCollider`))
            ;[1 1 1] Adjust and Clamp Rotation
            (bind _rotationtosetwheelto (`self.GetRotationFromHand`))
            ;[1 1 1] Set Lever Rotation X in Degrees
            (`SceneComponent.K2_SetWorldRotation` (`self.Lever`) (`KismetMathLibrary.TransformRotation` (`self.GetTransform`) (`KismetMathLibrary.MakeRotator` (`KismetMathLibrary.ClampAngle` _rotationtosetwheelto (* -1 (`self.MaxAngle`)) (* -1 (`self.MinAngle`))))) false false)
            (`self.IsGrabbedTickUpdate` DeltaSeconds)))
        (else
          (`self.IsUngrabbedTickUpdate` DeltaSeconds))))))

(event `self.ReceiveBeginPlay`
  (set `self.Colliders` (`SceneComponent.GetChildrenComponents` (`self.Lever`) false)))

(fn `GetClosestCollider`
  (params (ControllerReference :type "SceneComponent Object Reference"))
  (returns (FoundClosestCollider :type "SceneComponent Object Reference"))
  (locals (NewClosestColliderDist :type "Float (double-precision)") (NewClosestCollider :type "SceneComponent Object Reference"))
  (set `local.NewClosestColliderDist` 1000000.0)
  (set `local.NewClosestCollider` (`|GetArrayItem` (`self.Colliders`)))
  (for _array_element (`self.Colliders`)
    (bind _returnvalue (`KismetMathLibrary.Vector_Distance` (`SceneComponent.K2_GetComponentLocation` ControllerReference) (`SceneComponent.K2_GetComponentLocation` _array_element)))
    (if (< _returnvalue (`local.NewClosestColliderDist`))
      (bind _output_get (set `local.NewClosestCollider` _array_element))
      (set `local.NewClosestColliderDist` _returnvalue)))
  (return _output_get))

(fn `GetRatioFromIncrementedDegrees`
  (params (Degrees :type "Float (double-precision)"))
  (returns (Ratio :type "Float (double-precision)"))
  (bind _hingeincrement (`self.HingeIncrement`))
  (bind _returnvalue (`KismetMathLibrary.Conv_IntToDouble` (* (`KismetMathLibrary.FTrunc` (/ Degrees (`KismetMathLibrary.Conv_IntToDouble` _hingeincrement))) _hingeincrement)))
  (if (> Degrees 0.0)
    (return (/ _returnvalue (* -1 (`self.MaxAngle`))))
    (else
      (return (/ _returnvalue (`self.MinAngle`))))))

(fn `GetRawTurnAngleInDegrees`
  (returns (Angle :type "Float (double-precision)"))
  (return (.roll (`KismetMathLibrary.InverseTransformRotation` (`self.GetTransform`) (`SceneComponent.K2_GetComponentRotation` (`self.Lever`))))))

(fn `GetRotationFromHand`
  (returns (RotationToSetWheelTo :type "Float (double-precision)"))
  (bind _relativerotation (`self.GetRotationRelativeToWheel` (`self.ControllerScene`)))
  (return (- _relativerotation (`KismetMathLibrary.DegAtan2` (.y (`KismetMathLibrary.InverseTransformLocation` (`SceneComponent.K2_GetComponentToWorld` (`self.Lever`)) (`SceneComponent.K2_GetComponentLocation` (`self.ClosestCollider`)))) (.z (`KismetMathLibrary.InverseTransformLocation` (`SceneComponent.K2_GetComponentToWorld` (`self.Lever`)) (`SceneComponent.K2_GetComponentLocation` (`self.ClosestCollider`))))))))

(fn `GetRotationRelativeToWheel`
  (params (InputObject :type "SceneComponent Object Reference"))
  (returns (RelativeRotation :type "Float (double-precision)"))
  (return (`KismetMathLibrary.DegAtan2` (.y (`KismetMathLibrary.InverseTransformLocation` (`self.GetTransform`) (`SceneComponent.K2_GetComponentLocation` InputObject))) (.z (`KismetMathLibrary.InverseTransformLocation` (`self.GetTransform`) (`SceneComponent.K2_GetComponentLocation` InputObject))))))

(fn `GetTurnAngleInDegrees`
  (returns (Angle :type "Float (double-precision)"))
  (bind _angle (`self.GetRawTurnAngleInDegrees`))
  (if (>= 0.5 _angle)
    (return (`KismetMathLibrary.Conv_IntToDouble` (`KismetMathLibrary.FFloor` _angle)))
    (else
      (return (`KismetMathLibrary.Conv_IntToDouble` (`KismetMathLibrary.FCeil` _angle))))))

(fn `Grabbed`)

(fn `IsGrabbedTickUpdate`
  (params (DeltaTime :type "Float (double-precision)"))
  (return))

(fn `IsUngrabbedTickUpdate`
  (params (DeltaTime :type "Float (double-precision)")))

(fn `LetGoOf`)

(fn `TickUpdate`)

(fn `UpdateHandPositionToCollider`
  (params (MotionController :type "SceneComponent Object Reference") (Collider :type "SceneComponent Object Reference"))
  (`SceneComponent.K2_SetWorldLocationAndRotation` MotionController (`SceneComponent.K2_GetComponentLocation` Collider) (`SceneComponent.K2_GetComponentRotation` Collider) false false))

(fn `UserConstructionScript`)