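; A lever-system button variant that changes color to show whether it is fully pressed.
; On BeginPlay it creates and stores a dynamic material instance from the Button component's first material slot.
; The pressed-fully-down and released-from-full-down functions set that material's Color parameter to green and red respectively.
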(event `self.ReceiveBeginPlay`
  (`parent.ReceiveBeginPlay`)
  (bind _returnvalue (`PrimitiveComponent.CreateDynamicMaterialInstance` (`self.Button`) 0 null "None"))
  (set `self.colorMat` _returnvalue))

(fn `Button Was Released from Being Full Down`
  (`MaterialInstanceDynamic.SetVectorParameterValue` (`self.colorMat`) "Color" (struct :`R` 1.0 :`B` 0.046665 :`A` 1.0)))

(fn `ButtonWasPressedFullyDown`
  (`MaterialInstanceDynamic.SetVectorParameterValue` (`self.colorMat`) "Color" (struct :`R` 0.004252 :`G` 1.0 :`A` 1.0)))

(fn `UserConstructionScript`
  (`parent.UserConstructionScript`))