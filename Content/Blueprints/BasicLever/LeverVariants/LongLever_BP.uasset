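; Long lever variant of the basic lever, intended by its tick comment to drive ship speed from the lever's rotation.
; Tick update feeds the turn angle in degrees into the incremented-degree ratio function, without using the result in this graph.
; While ungrabbed, the lever eases back to zero roll through a delta-time-scaled lerp, converted from actor space to world rotation.
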(fn `IsUngrabbedTickUpdate`
  (params (DeltaTime :type "Float (double-precision)"))
  (bind _angle (`self.GetRawTurnAngleInDegrees`))
  (if (!= _angle 0.0)
    (`SceneComponent.K2_SetWorldRotation` (`self.Lever`) (`KismetMathLibrary.TransformRotation` (`self.GetTransform`) (`KismetMathLibrary.MakeRotator` (`KismetMathLibrary.Lerp` _angle 0.0 (* 5 DeltaTime)))) false false)))

(fn `TickUpdate`
  ;[1 1 1] Update Ship Speed based on Levers Rotation
  (bind _angle (`self.GetTurnAngleInDegrees`))
  (`self.GetRatioFromIncrementedDegrees` _angle))

(fn `UserConstructionScript`
  (`parent.UserConstructionScript`))