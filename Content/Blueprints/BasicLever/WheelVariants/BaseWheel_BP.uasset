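; Base grabbable wheel, built on the lever logic, that turns with the hand and keeps spinning when let go.
; UpdateSteeringRotation detects crossings of the 0/360 seam to accumulate total rotation from per-update deltas, then returns it clamped to min/max limits.
; On release the last delta becomes the spin speed, which the ungrabbed tick decelerates toward zero while feeding it through the same update to rotate the Lever.
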(fn `CheckIfRotationIsInMaxClampRange`
  (params (Rotation :type "Float (double-precision)"))
  (returns (IsInRange :type Boolean))
  (return (and (> Rotation (`self.MaxRotationClampRange`)) (<= Rotation 360.0))))

(fn `CheckIfRotationIsInMinClampRange`
  (params (Rotation :type "Float (double-precision)"))
  (returns (IsInRange :type Boolean))
  (return (and (< Rotation (`self.MinRotationClampRange`)) (>= Rotation 0.0))))

(fn `GetRotationFromHand`
  (returns (RotationToSetWheelTo :type "Float (double-precision)"))
  (bind _rotationtosetwheelto (`parent.GetRotationFromHand`))
  (bind _clampedcircularrotation (`self.Update Steering Rotation` _rotationtosetwheelto))
  (return _clampedcircularrotation))

(fn `Grabbed`
  (set `self.PreviousRotation` (`KismetMathLibrary.FClamp` (`self.PreviousRotation`) (`self.MinRotationClamp`) (`self.MaxRotationClamp`))))

(fn `IsUngrabbedTickUpdate`
  (params (DeltaTime :type "Float (double-precision)"))
  (bind _wheelspeedwhenletgo (`self.WheelSpeedWhenLetGo`))
  (if (> (`KismetMathLibrary.Abs` (`self.WheelSpeedWhenLetGo`)) 0.0)
    (if (> _wheelspeedwhenletgo 0.0)
      (set `self.WheelSpeedWhenLetGo` (`KismetMathLibrary.FClamp` (- (`self.WheelSpeedWhenLetGo`) (`self.WheelDecelerationAmount`)) 0.0 (`self.MaxWheelSpeedWhenLetGo`)))
      (else
        (set `self.WheelSpeedWhenLetGo` (`KismetMathLibrary.FClamp` (+ _wheelspeedwhenletgo (`self.WheelDecelerationAmount`)) (* -1 (`self.MaxWheelSpeedWhenLetGo`)) 0.0))))
    (bind _angle (`self.GetRawTurnAngleInDegrees`))
    (bind _clampedcircularrotation (`self.Update Steering Rotation` (+ _angle (`self.WheelSpeedWhenLetGo`))))
    (`SceneComponent.K2_SetWorldRotation` (`self.Lever`) (`KismetMathLibrary.TransformRotation` (`self.GetTransform`) (`KismetMathLibrary.MakeRotator` _clampedcircularrotation)) false false)))

(fn `LetGoOf`
  (set `self.WheelSpeedWhenLetGo` (`self.RotationDelta`)))

(fn `Update Steering Rotation`
  (params (DesiredRotation :type "Float (double-precision)"))
  (returns (ClampedCircularRotation :type "Float (double-precision)"))
  (bind _adjusteddesiredrotation (`self.AdjustedDesiredRotation`))
  (bind _returnvalue (- _adjusteddesiredrotation (`self.PreviousRotation`)))
  (bind _returnvalue_2 (+ (`self.TotalRotation`) (`self.RotationDelta`)))
  ;[0 0 0] Get Adjusted Rotation (Add under certain conditions)
  (`|ExecutionSequence`
    (:`then_0`
      (if (>= DesiredRotation 0.0)
        (set `self.AdjustedDesiredRotation` DesiredRotation)
        (else
          (set `self.AdjustedDesiredRotation` (+ DesiredRotation 360.0)))))
    (:`then_1`
      (bind _isinrange (`self.CheckIfRotationIsInMaxClampRange` (`self.PreviousRotation`)))
      (if _isinrange
        (bind _isinrange_2 (`self.CheckIfRotationIsInMinClampRange` (`self.AdjustedDesiredRotation`)))
        (else
          (bind _isinrange_3 (`self.CheckIfRotationIsInMinClampRange` (`self.PreviousRotation`)))
          (if _isinrange_3
            (bind _isinrange_4 (`self.CheckIfRotationIsInMaxClampRange` (`self.AdjustedDesiredRotation`)))))))
    (:`then_2`
      (if _isinrange_2
        (set `self.RotationDelta` (+ _returnvalue 360.0))
        (elif _isinrange_4
          (set `self.RotationDelta` (- _returnvalue 360.0))
          (else
            (set `self.RotationDelta` _returnvalue))))
      (set `self.PreviousRotation` _adjusteddesiredrotation)
      (if (> (`self.TotalRotation`) (+ (`self.MaxRotationClamp`) 360.0))
        (set `self.TotalRotation` (- _returnvalue_2 360.0))
        (elif (< (`self.TotalRotation`) (- (`self.MinRotationClamp`) 360.0))
          (set `self.TotalRotation` (+ _returnvalue_2 360.0))
          (else
            (set `self.TotalRotation` _returnvalue_2))))
      (bind _output_get (set `self.TotalClampedRotation` (`KismetMathLibrary.FClamp` (`self.TotalRotation`) (`self.MinRotationClamp`) (`self.MaxRotationClamp`))))
      (return _output_get))))

(fn `UserConstructionScript`)