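; BasicLever_BP is a VR lever actor that BP_MotionController can grab through Pickup and Drop events.
; Pickup attaches LeverRoot to the controller's component and sets InUse, while Drop calls DetachFromActor and clears it, both keeping world transforms.
; Tick is empty; disconnected nodes would snap LeverModel's roll to HingeIncrement steps to drive the Hinge's angular orientation target and print it.
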(event `/Game/Blueprints/PickupActorInterface.Pickup`
  (params (AttachTo :type "SceneComponent Object Reference"))
  (`SceneComponent.K2_AttachToComponent` (`self.LeverRoot`) AttachTo "None" "KeepWorld" "KeepWorld" "KeepWorld" false)
  (set `self.InUse` true))

(event `/Game/Blueprints/PickupActorInterface.Drop`
  (`self.K2_DetachFromActor` "KeepWorld" "KeepWorld" "KeepWorld")
  (set `self.InUse` false))

(event `self.ReceiveTick`
  (params (DeltaSeconds :type "Float (single-precision)")))

(fn `UserConstructionScript`)